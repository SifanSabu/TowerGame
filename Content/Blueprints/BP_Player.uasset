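; Player character for a 2D side-scrolling platformer, with Paper2D flipbook animation and Enhanced Input for movement, jump, dash and attacks.
; A forward trace while falling flags walljumps and damps velocity for wall friction.
; Dash launches along X with a temporary plane constraint and cooldown.
; Work in progress: input events set flipbooks directly, UpdateAnimation is disconnected, jump and E handlers are duplicated, and parry/pogo logic is partly unwired.
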(event `EnhancedInput|/Game/Input/Actions/IA_Attack1`
  (params (ActionValue :type Boolean) (ElapsedSeconds :type "Float (double-precision)") (TriggeredSeconds :type "Float (double-precision)") (InputAction :type "InputAction Object Reference" :default "/Game/Input/Actions/IA_Attack1.IA_Attack1"))
  (:`Triggered`
    (if (not (`self.IsAttacking`))
      (set `self.IsAttacking` true)
      (`KismetSystemLibrary.Delay` 0.5)
      (set `self.IsAttacking` false))))

(event `self.ReceiveBeginPlay`
  (bind _asplayer_controller (cast `PlayerController` (`self.GetController`)))
  (`EnhancedInputSubsystemInterface.AddMappingContext` (pcsubsystem `EnhancedInputLocalPlayerSubsystem` _asplayer_controller) "/Game/Input/IMC_Platforming.IMC_Platforming" 0 (struct)))

(event `Reset Pogo`
  (`/Engine/EditorBlueprintResources/StandardMacros.DoOnce` false :!via `Reset`
    (:`Completed`
      (`self.LaunchCharacter` (0.0 0.0 1000.0) false true)
      (`KismetSystemLibrary.Delay` 0.3)
      (set `self.IsParrying` false)
      (`KismetSystemLibrary.PrintString` "fucky there"))))

(event `EnhancedInput|/Game/Input/Actions/IA_Jump`
  (params (ActionValue :type Boolean) (ElapsedSeconds :type "Float (double-precision)") (TriggeredSeconds :type "Float (double-precision)") (InputAction :type "InputAction Object Reference" :default "/Game/Input/Actions/IA_Jump.IA_Jump"))
  (bind (_returnvalue_roll _returnvalue_pitch _returnvalue_yaw) (`KismetMathLibrary.BreakRotator` (`self.K2_GetActorRotation`)))
  (:`Started`
    (if (`self.WalljumpCheck`)
      (`self.LaunchCharacter` (+ (* (`self.GetActorForwardVector`) (`self.WalljumpForce`)) (0.0 0.0 1000.0)) true true)
      (`self.K2_SetActorRotation` (`KismetMathLibrary.MakeRotator` (+ 0.0 _returnvalue_roll) _returnvalue_pitch _returnvalue_yaw))
      (else
        (`self.Jump`))))
  (:`Completed`
    (`self.StopJumping`)))

(event `self.ReceiveTick`
  (params (DeltaSeconds :type "Float (single-precision)"))
  (bind _capsulecomponent (`self.CapsuleComponent`))
  (bind _charactermovement (`self.CharacterMovement`))
  (bind _returnvalue (`SceneComponent.K2_GetComponentLocation` _capsulecomponent))
  (if (`NavMovementInterface.IsFalling` (`self.CharacterMovement`))
    (bind (_outhit _returnvalue_2) (`KismetSystemLibrary.LineTraceSingle` :`Start` _returnvalue :`End` (+ _returnvalue (* (`SceneComponent.GetForwardVector` _capsulecomponent) (`self.DistanceToWallCheck`))) :`TraceChannel` "TraceTypeQuery3" :`DrawDebugType` "ForDuration"))
    (if _returnvalue_2
      (set `self.WalljumpCheck` true)
      (set `MovementComponent.Velocity` (`KismetMathLibrary.VInterpTo_Constant` (`MovementComponent.Velocity` _charactermovement) (0.0 0.0 0.0) (`GameplayStatics.GetWorldDeltaSeconds`) 5000.0) _charactermovement)
      (else
        (set `self.WalljumpCheck` false :!label _label)))
    (else
      (goto _label))))

(event `EnhancedInput|/Game/Input/Actions/IA_Attack2`
  (params (ActionValue :type Boolean) (ElapsedSeconds :type "Float (double-precision)") (TriggeredSeconds :type "Float (double-precision)") (InputAction :type "InputAction Object Reference" :default "/Game/Input/Actions/IA_Attack2.IA_Attack2"))
  (:`Triggered`
    (if (not (`self.IsParrying`))
      (set `self.IsParrying` true))))

(event `Key|E`
  (params (Key :type "Key Structure"))
  (:`Pressed`
    (`PaperFlipbookComponent.SetFlipbook` (`self.Sprite`) "/Game/PaperAssets/Character/Flipbooks/FB_Player_Attack3.FB_Player_Attack3")
    (`PaperFlipbookComponent.SetLooping` (`self.Sprite`) false)))

(event `self.Sprite.OnFinishedPlaying`
  (`PaperFlipbookComponent.SetFlipbook` (`self.Sprite`) "/Game/PaperAssets/Character/Flipbooks/FB_Player_Idle1.FB_Player_Idle1")
  (`PaperFlipbookComponent.SetLooping` (`self.Sprite`) true)
  (if (not (`PaperFlipbookComponent.IsPlaying` (`self.Sprite`)))
    (`PaperFlipbookComponent.Play` (`self.Sprite`))))

(event `EnhancedInput|/Game/Input/Actions/IA_Jump`
  (params (ActionValue :type Boolean) (ElapsedSeconds :type "Float (double-precision)") (TriggeredSeconds :type "Float (double-precision)") (InputAction :type "InputAction Object Reference" :default "/Game/Input/Actions/IA_Jump.IA_Jump"))
  ; This needs to be handled differently
  (:`Started`
    (`self.Jump`)
    (if (not true)
      (set `self.IsJumping` true)
      (`PaperFlipbookComponent.SetFlipbook` (`self.Sprite`) "/Game/PaperAssets/Character/Flipbooks/FB_Player_Jump1.FB_Player_Jump1")))
  (:`Completed`
    (`self.StopJumping`)
    (`PaperFlipbookComponent.SetFlipbook` (`self.Sprite`) "/Game/PaperAssets/Character/Flipbooks/FB_Player_Fall1.FB_Player_Fall1")))

(event `EnhancedInput|/Game/Input/Actions/IA_Move`
  (params (ActionValue :type "Float (double-precision)") (ElapsedSeconds :type "Float (double-precision)") (TriggeredSeconds :type "Float (double-precision)") (InputAction :type "InputAction Object Reference" :default "/Game/Input/Actions/IA_Move.IA_Move"))
  (:`Triggered`
    ; This needs to be handled differently
    (`self.AddMovementInput` (1.0 0.0 0.0) ActionValue)
    (`Controller.SetControlRotation` (`self.GetController`) (select `bool` (> ActionValue 0.0) :`false` (`KismetMathLibrary.MakeRotator` 0.0 0.0 180.0) :`true` (`KismetMathLibrary.MakeRotator` 0.0)))
    (if (> (`KismetMathLibrary.VSize` (`self.GetVelocity`)) 0.0)
      (if (`NavMovementComponent.IsMovingOnGround` (`self.CharacterMovement`))
        (if (== (`KismetMathLibrary.VSize` (`self.GetVelocity`)) 0.0)
          (`PaperFlipbookComponent.SetFlipbook` (`self.Sprite`) "/Game/PaperAssets/Character/Flipbooks/FB_Player_Jump1.FB_Player_Jump1")
          (else
            (`PaperFlipbookComponent.SetFlipbook` (`self.Sprite`) "/Game/PaperAssets/Character/Flipbooks/FB_Player_Run1.FB_Player_Run1")
            (if (`self.IsDashing`)
              (`PaperFlipbookComponent.SetFlipbook` (`self.Sprite`) "/Game/PaperAssets/Character/Flipbooks/FB_Player_Fall1.FB_Player_Fall1")
              (if (`NavMovementComponent.IsMovingOnGround` (`self.CharacterMovement`))
                (`PaperFlipbookComponent.SetFlipbook` (`self.Sprite`) "/Game/PaperAssets/Character/Flipbooks/FB_Player_Run1.FB_Player_Run1")
                (set `self.IsDashing` false)))))
        (else
          (`PaperFlipbookComponent.SetFlipbook` (`self.Sprite`) "/Game/PaperAssets/Character/Flipbooks/FB_Player_Fall1.FB_Player_Fall1")))))
  (:`Completed`
    (`PaperFlipbookComponent.SetFlipbook` (`self.Sprite`) "/Game/PaperAssets/Character/Flipbooks/FB_Player_Idle1.FB_Player_Idle1")))

(event `Key|E`
  (params (Key :type "Key Structure"))
  (bind _sprite (`self.Sprite`))
  (:`Pressed`
    (`PaperFlipbookComponent.SetFlipbook` _sprite "/Game/PaperAssets/Character/Flipbooks/FB_Player_Attack1.FB_Player_Attack1")
    (`PaperFlipbookComponent.SetLooping` _sprite false)))

(event `EnhancedInput|/Game/Input/Actions/IA_Dash`
  (params (ActionValue :type Boolean) (ElapsedSeconds :type "Float (double-precision)") (TriggeredSeconds :type "Float (double-precision)") (InputAction :type "InputAction Object Reference" :default "/Game/Input/Actions/IA_Dash.IA_Dash"))
  (bind (_returnvalue_x _returnvalue_y _returnvalue_z) (`KismetMathLibrary.BreakVector` (`self.K2_GetActorLocation`)))
  (bind _charactermovement (`self.CharacterMovement`))
  (bind _charactermovement_2 (`self.CharacterMovement`))
  (bind _returnvalue_x_2 (`KismetMathLibrary.BreakVector` (* (`self.GetVelocity`) 1.0)))
  (bind _returnvalue_x_3 (`KismetMathLibrary.BreakVector` (* (`self.GetActorForwardVector`) (1.0 0.0 0.0))))
  (bind _returnvalue_x_4 (`KismetMathLibrary.BreakVector` (* (`self.GetVelocity`) 1.0)))
  (:`Triggered`
    (if (not (`self.IsDashing`))
      (set `self.IsDashing` true)
      (`PaperFlipbookComponent.SetFlipbook` (`self.Sprite`) "/Game/PaperAssets/Character/Flipbooks/FB_Player_Jump1.FB_Player_Jump1")
      (`MovementComponent.SetPlaneConstraintNormal` (`self.CharacterMovement`) (`KismetMathLibrary.MakeVector` 0.0 0.0 _returnvalue_z))
      (if (> _returnvalue_x_3 0.0)
        (`self.LaunchCharacter` (`KismetMathLibrary.MakeVector` (+ _returnvalue_x_2 2500.0)))
        (`KismetSystemLibrary.Delay` 0.2)
        (`MovementComponent.StopMovementImmediately` _charactermovement_2)
        (`MovementComponent.SetPlaneConstraintNormal` _charactermovement_2 (0.0 0.0 0.0))
        (`KismetSystemLibrary.Delay` 1.0)
        (set `self.IsDashing` false)
        (else
          (`self.LaunchCharacter` (`KismetMathLibrary.MakeVector` (+ _returnvalue_x_4 -2500.0)))
          (`KismetSystemLibrary.Delay` 0.2)
          (`MovementComponent.StopMovementImmediately` _charactermovement)
          (`MovementComponent.SetPlaneConstraintNormal` _charactermovement (0.0 0.0 0.0))
          (`KismetSystemLibrary.Delay` 1.0)
          (set `self.IsDashing` false))))))

(fn `UpdateAnimation`
  (bind (_returnvalue_x _returnvalue_y _returnvalue_z) (`KismetMathLibrary.BreakVector` (`self.GetVelocity`)))
  (if (`self.IsAttacking`)
    (`PaperFlipbookComponent.SetFlipbook` (`self.Sprite`) "/Game/PaperAssets/Character/Flipbooks/FB_Player_Attack1.FB_Player_Attack1")
    (elif (`self.IsParrying`)
      (`PaperFlipbookComponent.SetFlipbook` (`self.Sprite`) "/Game/PaperAssets/Character/Flipbooks/FB_Player_Attack3.FB_Player_Attack3")
      (`PaperFlipbookComponent.SetLooping` (`self.Sprite`) false)
      (elif (`NavMovementComponent.IsMovingOnGround` (`self.CharacterMovement`))
        (if (> (`KismetMathLibrary.VSize` (`self.GetVelocity`)) 0.0)
          (`PaperFlipbookComponent.SetFlipbook` (`self.Sprite`) "/Game/PaperAssets/Character/Flipbooks/FB_Player_Run1.FB_Player_Run1")
          (else
            (`PaperFlipbookComponent.SetFlipbook` (`self.Sprite`) "/Game/PaperAssets/Character/Flipbooks/FB_Player_Idle1.FB_Player_Idle1")))
        (elif (< _returnvalue_z -100.0)
          (`PaperFlipbookComponent.SetFlipbook` (`self.Sprite`) "/Game/PaperAssets/Character/Flipbooks/FB_Player_Fall1.FB_Player_Fall1")
          (else
            (`PaperFlipbookComponent.SetFlipbook` (`self.Sprite`) "/Game/PaperAssets/Character/Flipbooks/FB_Player_Jump1.FB_Player_Jump1")))))))

(fn `UserConstructionScript`)